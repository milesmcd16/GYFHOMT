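; Game mode that runs a wave-based round loop of spawning enemies and waiting until all are gone.
; RoundStart passes the round number to every EnemySpawnerMk2, removes WBP_enterstuff widgets, then flags the round active after a delay.
; While active, Tick polls for EnemyABSTRACT actors; when none remain, TylerWorriesTooMuch increments the round, shows WBP_enterstuff and calls RoundStart on the Jank actor.
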(event `Tyler worries too much`
  (set `self.localizedround#` (+ (`self.localizedround#`) 1))
  (bind _returnvalue (`|CreateWidget` "/Game/ui/WBP_enterstuff.WBP_enterstuff_C"))
  (`UserWidget.AddToViewport` _returnvalue 0)
  (bind _returnvalue_2 (`GameplayStatics.GetActorOfClass` "/Game/ui/jank.jank_C"))
  (`/Game/ui/jank.RoundStart` _returnvalue_2))

(event `RoundStart`
  (if (not (`self.roundstarted`))
    (bind _outactors (`GameplayStatics.GetAllActorsOfClass` "/Game/Blueprints/Enemies/EnemySpawnerMk2.EnemySpawnerMk2_C"))
    (for _array_element _outactors
      (`/Game/Blueprints/Enemies/EnemySpawnerMk2.enemiestospawnya` _array_element (`self.localizedround#`)))
    (bind _foundwidgets (`WidgetBlueprintLibrary.GetAllWidgetsOfClass` "/Game/ui/WBP_enterstuff.WBP_enterstuff_C"))
    (`Widget.RemoveFromParent` _foundwidgets)
    (`KismetSystemLibrary.Delay` 5.0)
    (set `self.roundstarted` true)))

(event `self.ReceiveTick`
  (params (DeltaSeconds :type "Float (single-precision)"))
  (if (`self.roundstarted`)
    (bind _outactors (`GameplayStatics.GetAllActorsOfClass` "/Game/Blueprints/Enemies/Actors/EnemyABSTRACT.EnemyABSTRACT_C"))
    (if (== (`KismetArrayLibrary.Array_Length` _outactors) 0)
      (`self.Tyler worries too much`)
      (set `self.roundstarted` false))))

(fn `UserConstructionScript`)