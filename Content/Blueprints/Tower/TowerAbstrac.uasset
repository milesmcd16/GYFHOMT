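; Abstract tower base that tracks enemies inside its vision radius and feeds a target to its AI blackboard.
; Overlap events maintain an EnemiesInVision list; an enemy entering an empty list becomes the target, and any enemy leaving clears that target without choosing another.
; BeginPlay sets the line-of-sight key to true, and Tick polls a ShowRange click flag to toggle the range display's visibility.
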(event `self.ReceiveBeginPlay`
  (`BlackboardComponent.SetValueAsBool` (`self.MyTowerBlackboard`) (`self.LOSKey`) true))

(event `self.ReceiveTick`
  (params (DeltaSeconds :type "Float (single-precision)"))
  (if (`/Game/Blueprints/ActorComponents/Clickable.WasClicked` (`self.ShowRange`))
    (`SceneComponent.ToggleVisibility` (`self.Range`) false)))

(event `self.Vision Radius.OnComponentBeginOverlap`
  (params (OverlappedComponent :type "PrimitiveComponent Object Reference") (OtherActor :type "Actor Object Reference") (OtherComp :type "PrimitiveComponent Object Reference") (OtherBodyIndex :type Integer) (bFromSweep :type Boolean) (SweepResult :type "HitResult Structure (by ref)"))
  (bind _empty (`self.IsEmpty`))
  (bind _asenemy_abstract (cast `/Game/Blueprints/Enemies/Actors/EnemyABSTRACT` OtherActor))
  (`KismetArrayLibrary.Array_Add` (`self.Enemies In Vision`) _asenemy_abstract)
  (if _empty
    (`BlackboardComponent.SetValueAsObject` (`AIBlueprintHelperLibrary.GetBlackboard` (`self.GetController`)) (`self.targetName`) _asenemy_abstract)))

(event `self.Vision Radius.OnComponentEndOverlap`
  (params (OverlappedComponent :type "PrimitiveComponent Object Reference") (OtherActor :type "Actor Object Reference") (OtherComp :type "PrimitiveComponent Object Reference") (OtherBodyIndex :type Integer))
  (bind _asenemy_abstract (cast `/Game/Blueprints/Enemies/Actors/EnemyABSTRACT` OtherActor))
  (`KismetArrayLibrary.Array_RemoveItem` (`self.Enemies In Vision`) _asenemy_abstract)
  (`BlackboardComponent.SetValueAsObject` (`AIBlueprintHelperLibrary.GetBlackboard` (`self.GetController`)) (`self.targetName`) null))

(fn `IsEmpty`
  (returns (Empty :type Boolean))
  (return (== (`KismetArrayLibrary.Array_Length` (`self.Enemies In Vision`)) 0)))

(fn `UserConstructionScript`)