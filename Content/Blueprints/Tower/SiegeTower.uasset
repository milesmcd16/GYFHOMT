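; Siege tower AI pawn that targets enemies within a ring, excluding those too close.
; Outer and inner overlap volumes add and remove EnemyABSTRACT actors in TargetList and update the EnemyInRange blackboard key.
; BeginPlay, ResetCD and ReduceCD write the cooldown to the blackboard, in full or scaled by a percent.
; Tick polls the ShowRange clicked flag to toggle both range visuals.
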(event `self.ReceiveBeginPlay`
  (`BlackboardComponent.SetValueAsFloat` (`AIBlueprintHelperLibrary.GetBlackboard` (`self.GetController`)) (`self.cdName`) (`self.CDTime`)))

(event `ResetCD`
  (`BlackboardComponent.SetValueAsFloat` (`AIBlueprintHelperLibrary.GetBlackboard` (`self.GetController`)) (`self.cdName`) (`self.CDTime`)))

(event `ReduceCD`
  (params (percent :type "Float (double-precision)"))
  (`BlackboardComponent.SetValueAsFloat` (`AIBlueprintHelperLibrary.GetBlackboard` (`self.GetController`)) (`self.cdName`) (* percent (`self.CDTime`))))

(event `self.ReceiveTick`
  (params (DeltaSeconds :type "Float (single-precision)"))
  (if (`/Game/Blueprints/ActorComponents/Clickable.WasClicked` (`self.ShowRange`))
    (`SceneComponent.ToggleVisibility` (`self.InnerRange`) false)
    (`SceneComponent.ToggleVisibility` (`self.Range`) false)))

(event `self.OuterLimit.OnComponentBeginOverlap`
  (params (OverlappedComponent :type "PrimitiveComponent Object Reference") (OtherActor :type "Actor Object Reference") (OtherComp :type "PrimitiveComponent Object Reference") (OtherBodyIndex :type Integer) (bFromSweep :type Boolean) (SweepResult :type "HitResult Structure (by ref)"))
  (bind _asenemy_abstract (cast `/Game/Blueprints/Enemies/Actors/EnemyABSTRACT` OtherActor))
  (`KismetArrayLibrary.Array_Add` (`self.TargetList`) _asenemy_abstract)
  (`BlackboardComponent.SetValueAsBool` (`AIBlueprintHelperLibrary.GetBlackboard` (`self.GetController`)) (`self.EnemyInRange`) true))

(event `self.InnerLimit.OnComponentBeginOverlap`
  (params (OverlappedComponent :type "PrimitiveComponent Object Reference") (OtherActor :type "Actor Object Reference") (OtherComp :type "PrimitiveComponent Object Reference") (OtherBodyIndex :type Integer) (bFromSweep :type Boolean) (SweepResult :type "HitResult Structure (by ref)"))
  (bind _targetlist (`self.TargetList`))
  (bind _asenemy_abstract (cast `/Game/Blueprints/Enemies/Actors/EnemyABSTRACT` OtherActor))
  (`KismetArrayLibrary.Array_RemoveItem` _targetlist _asenemy_abstract)
  (if (== (`KismetArrayLibrary.Array_Length` _targetlist) 0)
    (`BlackboardComponent.SetValueAsBool` (`AIBlueprintHelperLibrary.GetBlackboard` (`self.GetController`)) (`self.EnemyInRange`) false)))

(event `self.InnerLimit.OnComponentEndOverlap`
  (params (OverlappedComponent :type "PrimitiveComponent Object Reference") (OtherActor :type "Actor Object Reference") (OtherComp :type "PrimitiveComponent Object Reference") (OtherBodyIndex :type Integer))
  (bind _asenemy_abstract (cast `/Game/Blueprints/Enemies/Actors/EnemyABSTRACT` OtherActor))
  (`KismetArrayLibrary.Array_Add` (`self.TargetList`) _asenemy_abstract)
  (`BlackboardComponent.SetValueAsBool` (`AIBlueprintHelperLibrary.GetBlackboard` (`self.GetController`)) (`self.EnemyInRange`) true))

(event `self.OuterLimit.OnComponentEndOverlap`
  (params (OverlappedComponent :type "PrimitiveComponent Object Reference") (OtherActor :type "Actor Object Reference") (OtherComp :type "PrimitiveComponent Object Reference") (OtherBodyIndex :type Integer))
  (bind _targetlist (`self.TargetList`))
  (bind _asenemy_abstract (cast `/Game/Blueprints/Enemies/Actors/EnemyABSTRACT` OtherActor))
  (`KismetArrayLibrary.Array_RemoveItem` _targetlist _asenemy_abstract)
  (if (== (`KismetArrayLibrary.Array_Length` _targetlist) 0)
    (`BlackboardComponent.SetValueAsBool` (`AIBlueprintHelperLibrary.GetBlackboard` (`self.GetController`)) (`self.EnemyInRange`) false)))

(fn `UserConstructionScript`)