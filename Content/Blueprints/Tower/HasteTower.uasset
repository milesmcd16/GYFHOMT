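; Haste tower that speeds up nearby towers by cutting their cooldowns.
; On BeginPlay it nudges its snow crystal meshes up then back down in two loops, then calls ReduceCD on overlapping towers through a chain of casts to each tower class.
; The buff is a one-time pass, as the overlap events are empty.
; Tick toggles the Range visual while the Clickable reports a click.
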(event `self.ReceiveTick`
  (params (DeltaSeconds :type "Float (single-precision)"))
  (if (`/Game/Blueprints/ActorComponents/Clickable.WasClicked` (`self.Clickable`))
    (`SceneComponent.ToggleVisibility` (`self.Range`) false)))

(event `self.ReceiveBeginPlay`
  (for _ (`self.NewVar_0`)
    (`SceneComponent.K2_AddRelativeLocation` (`self.snow_detail_crystal_snow_detail_crystal7`) (0.0 0.0 1.0) false false)
    (`SceneComponent.K2_AddRelativeLocation` (`self.snow_detail_crystal_snow_detail_crystal6`) (0.0 0.0 1.0) false false)
    (`SceneComponent.K2_AddRelativeLocation` (`self.snow_detail_crystal_snow_detail_crystal5`) (0.0 0.0 1.0) false false)
    (`SceneComponent.K2_AddRelativeLocation` (`self.snow_detail_crystal_snow_detail_crystal4`) (0.0 0.0 1.0) false false)
    (`SceneComponent.K2_AddRelativeLocation` (`self.snow_detail_crystal_snow_detail_crystal3`) (0.0 0.0 1.0) false false)
    (`SceneComponent.K2_AddRelativeLocation` (`self.snow_detail_crystal_snow_detail_crystal2`) (0.0 0.0 1.0) false false)
    (`SceneComponent.K2_AddRelativeLocation` (`self.snow_detail_crystal_snow_detail_crystal1`) (0.0 0.0 1.0) false false)
    (`SceneComponent.K2_AddRelativeLocation` (`self.snow_detail_crystal_snow_detail_crystal`) (0.0 0.0 1.0) false false))
  (for _ (`self.NewVar_0`)
    (`SceneComponent.K2_AddRelativeLocation` (`self.snow_detail_crystal_snow_detail_crystal7`) (0.0 0.0 -1.0) false false)
    (`SceneComponent.K2_AddRelativeLocation` (`self.snow_detail_crystal_snow_detail_crystal6`) (0.0 0.0 -1.0) false false)
    (`SceneComponent.K2_AddRelativeLocation` (`self.snow_detail_crystal_snow_detail_crystal5`) (0.0 0.0 -1.0) false false)
    (`SceneComponent.K2_AddRelativeLocation` (`self.snow_detail_crystal_snow_detail_crystal4`) (0.0 0.0 -1.0) false false)
    (`SceneComponent.K2_AddRelativeLocation` (`self.snow_detail_crystal_snow_detail_crystal3`) (0.0 0.0 -1.0) false false)
    (`SceneComponent.K2_AddRelativeLocation` (`self.snow_detail_crystal_snow_detail_crystal2`) (0.0 0.0 -1.0) false false)
    (`SceneComponent.K2_AddRelativeLocation` (`self.snow_detail_crystal_snow_detail_crystal1`) (0.0 0.0 -1.0) false false)
    (`SceneComponent.K2_AddRelativeLocation` (`self.snow_detail_crystal_snow_detail_crystal`) (0.0 0.0 -1.0) false false))
  (for _array_element (`PrimitiveComponent.GetOverlappingActors` (`self.Myrange`) null)
    (bind _astower_abstrac (cast `/Game/Blueprints/Tower/TowerAbstrac` _array_element)
      (:`then`
        (`/Game/Blueprints/Tower/TowerAbstrac.ReduceCD` _astower_abstrac 0.7))
      (:`CastFailed`
        (bind _asfireball_tower (cast `/Game/Blueprints/Tower/FireballTower` _array_element)
          (:`then`
            (`/Game/Blueprints/Tower/FireballTower.ReduceCD` _asfireball_tower 0.7))
          (:`CastFailed`
            (bind _assiege_tower (cast `/Game/Blueprints/Tower/SiegeTower` _array_element)
              (:`then`
                (`/Game/Blueprints/Tower/SiegeTower.ReduceCD` _assiege_tower 0.7))
              (:`CastFailed`
                (bind _assludge_tower (cast `/Game/Blueprints/Tower/SludgeTower` _array_element))
                (`KismetSystemLibrary.PrintString` "Hello")
                (`/Game/Blueprints/Tower/SludgeTower.ReduceCD` _assludge_tower 0.7)))))))))

(event `self.Myrange.OnComponentBeginOverlap`
  (params (OverlappedComponent :type "PrimitiveComponent Object Reference") (OtherActor :type "Actor Object Reference") (OtherComp :type "PrimitiveComponent Object Reference") (OtherBodyIndex :type Integer) (bFromSweep :type Boolean) (SweepResult :type "HitResult Structure (by ref)")))

(event `self.Myrange.OnComponentEndOverlap`
  (params (OverlappedComponent :type "PrimitiveComponent Object Reference") (OtherActor :type "Actor Object Reference") (OtherComp :type "PrimitiveComponent Object Reference") (OtherBodyIndex :type Integer)))

(fn `UserConstructionScript`)