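; Tower base Blueprint that acts as a clickable slot for placing a tower through a shop menu.
; Tick polls Clickable.WasClicked; when it and CanSpawnAtBase are true, the mesh turns glass and a new WBP_TowerShop opens with keyboard focus and this base as SelectedTowerBase.
; The walnut material returns whenever WasClicked is false.
; ShopOpen is set but never checked here, so nothing in this graph guards against repeated widget creation.
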(event `self.ReceiveTick`
  (params (DeltaSeconds :type "Float (single-precision)"))
  ;[1 1 1] checks if the tower base mesh is clicked and if it is and theres not a tower there already it opens the topwer shop
  (if (`/Game/Blueprints/ActorComponents/Clickable.WasClicked` (`self.Clickable`))
    (if (`self.CanSpawnAtBase`)
      (`PrimitiveComponent.SetMaterial` (`self.StaticMesh`) 0 "/Game/Map/glass.glass")
      (bind _returnvalue (`|CreateWidget` "/Game/ui/WBP_TowerSHop.WBP_TowerShop_C"))
      (set `self.ShopOpen` true)
      (`UserWidget.AddToViewport` _returnvalue 0)
      (`Widget.SetKeyboardFocus` _returnvalue)
      (set `/Game/ui/WBP_TowerSHop.SelectedTowerBase` self _returnvalue))
    (else
      (`PrimitiveComponent.SetMaterial` (`self.StaticMesh`) 0 "/Game/StarterContent/Materials/M_Wood_Walnut.M_Wood_Walnut"))))

(fn `UserConstructionScript`)