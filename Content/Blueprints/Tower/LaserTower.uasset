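; Laser tower that tracks enemies inside its HitBox and reports them to its AI controller's Blackboard.
; Overlap events add and remove EnemyABSTRACT actors in EnemiesInRange, setting Target when IsEmpty passes on entry and clearing it whenever any enemy leaves.
; Tick writes the IsEmpty result straight into the EnemyInRange key, so that key is true when no enemies are in range.
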(event `self.ReceiveTick`
  (params (DeltaSeconds :type "Float (single-precision)"))
  (bind _empty (`self.IsEmpty`))
  (`BlackboardComponent.SetValueAsBool` (`AIBlueprintHelperLibrary.GetBlackboard` (`self.GetController`)) (`self.EnemyInRange`) _empty))

(event `self.HitBox.OnComponentBeginOverlap`
  (params (OverlappedComponent :type "PrimitiveComponent Object Reference") (OtherActor :type "Actor Object Reference") (OtherComp :type "PrimitiveComponent Object Reference") (OtherBodyIndex :type Integer) (bFromSweep :type Boolean) (SweepResult :type "HitResult Structure (by ref)"))
  (bind _empty (`self.IsEmpty`))
  (bind _asenemy_abstract (cast `/Game/Blueprints/Enemies/Actors/EnemyABSTRACT` OtherActor))
  (`KismetArrayLibrary.Array_Add` (`self.EnemiesInRange`) _asenemy_abstract)
  (if _empty
    (`BlackboardComponent.SetValueAsObject` (`AIBlueprintHelperLibrary.GetBlackboard` (`self.GetController`)) (`self.Target`) _asenemy_abstract)))

(event `self.HitBox.OnComponentEndOverlap`
  (params (OverlappedComponent :type "PrimitiveComponent Object Reference") (OtherActor :type "Actor Object Reference") (OtherComp :type "PrimitiveComponent Object Reference") (OtherBodyIndex :type Integer))
  (bind _asenemy_abstract (cast `/Game/Blueprints/Enemies/Actors/EnemyABSTRACT` OtherActor))
  (`KismetArrayLibrary.Array_RemoveItem` (`self.EnemiesInRange`) _asenemy_abstract)
  (`BlackboardComponent.SetValueAsObject` (`AIBlueprintHelperLibrary.GetBlackboard` (`self.GetController`)) (`self.Target`) null))

(fn `IsEmpty`
  (returns (Empty :type Boolean))
  (return (== (`KismetArrayLibrary.Array_Length` (`self.EnemiesInRange`)) 0)))

(fn `UserConstructionScript`)