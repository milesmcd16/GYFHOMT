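; Ballista tower, an AI-controlled tower that tracks enemies in range and feeds combat state to its controller's blackboard.
; Range overlaps maintain the enemy list and set the line-of-sight key, which clears once the list empties.
; BeginPlay seeds the cooldown and Ballista projectile class, with events to reset or scale the cooldown.
; Tick toggles the range indicator's visibility while ShowRange's clicked flag is set.
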(event `ResetCD`
  (`BlackboardComponent.SetValueAsFloat` (`AIBlueprintHelperLibrary.GetBlackboard` (`self.GetController`)) (`self.cdName`) (`self.CDTimer`)))

(event `ReduceCD`
  (params (percent :type "Float (double-precision)"))
  (`BlackboardComponent.SetValueAsFloat` (`AIBlueprintHelperLibrary.GetBlackboard` (`self.GetController`)) (`self.cdName`) (* percent (`self.CDTimer`))))

(event `self.ReceiveBeginPlay`
  (bind _returnvalue (`AIBlueprintHelperLibrary.GetBlackboard` (`self.GetController`)))
  (`BlackboardComponent.SetValueAsBool` _returnvalue (`self.LOSKey`) false)
  (`BlackboardComponent.SetValueAsFloat` _returnvalue (`self.cdName`) (`self.CDTimer`))
  (`BlackboardComponent.SetValueAsClass` _returnvalue (`self.Projectile`) "/Game/Blueprints/Tower/Projectiles/Ballista/Ballista.Ballista_C"))

(event `self.ReceiveTick`
  (params (DeltaSeconds :type "Float (single-precision)"))
  (if (`/Game/Blueprints/ActorComponents/Clickable.WasClicked` (`self.ShowRange`))
    (`SceneComponent.ToggleVisibility` (`self.Range`) false)))

(event `self.MyRange.OnComponentBeginOverlap`
  (params (OverlappedComponent :type "PrimitiveComponent Object Reference") (OtherActor :type "Actor Object Reference") (OtherComp :type "PrimitiveComponent Object Reference") (OtherBodyIndex :type Integer) (bFromSweep :type Boolean) (SweepResult :type "HitResult Structure (by ref)"))
  (bind _asenemy_abstract (cast `/Game/Blueprints/Enemies/Actors/EnemyABSTRACT` OtherActor))
  (`KismetArrayLibrary.Array_Add` (`self.EnemyList`) _asenemy_abstract)
  (`BlackboardComponent.SetValueAsBool` (`AIBlueprintHelperLibrary.GetBlackboard` (`self.GetController`)) (`self.LOSKey`) true))

(event `self.MyRange.OnComponentEndOverlap`
  (params (OverlappedComponent :type "PrimitiveComponent Object Reference") (OtherActor :type "Actor Object Reference") (OtherComp :type "PrimitiveComponent Object Reference") (OtherBodyIndex :type Integer))
  (bind _enemylist (`self.EnemyList`))
  (bind _asenemy_abstract (cast `/Game/Blueprints/Enemies/Actors/EnemyABSTRACT` OtherActor))
  (`KismetArrayLibrary.Array_RemoveItem` _enemylist _asenemy_abstract)
  (if (== (`KismetArrayLibrary.Array_Length` _enemylist) 0)
    (`BlackboardComponent.SetValueAsBool` (`AIBlueprintHelperLibrary.GetBlackboard` (`self.GetController`)) (`self.LOSKey`) false)))

(fn `UserConstructionScript`)