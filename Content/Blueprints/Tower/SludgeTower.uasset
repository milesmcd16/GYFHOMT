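; Sludge tower Blueprint with a player-toggled range display that sets the target location for its AI controller.
; On BeginPlay it disables clicking on the RangeDef child actor and sets RoundStarted in the blackboard.
; Tick polls ShowRange clicks to toggle Range visibility and clickability together.
; Hiding the range writes the RangeDef's selected world location to the blackboard's Target key as a vector.
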(event `UpdateTarget`
  (bind _asrange_def (cast `/Game/Blueprints/Tower/Range/RangeDef` (`ChildActorComponent.ChildActor` (`self.Range`))))
  (`BlackboardComponent.SetValueAsVector` (`AIBlueprintHelperLibrary.GetBlackboard` (`self.GetController`)) (`self.Target`) (`SceneComponent.K2_GetComponentLocation` (`/Game/Blueprints/Tower/Range/RangeDef.Selected` _asrange_def))))

(event `self.ReceiveBeginPlay`
  (bind _asrange_def (cast `/Game/Blueprints/Tower/Range/RangeDef` (`ChildActorComponent.ChildActor` (`self.Range`))))
  (`/Game/Blueprints/Tower/Range/RangeDef.SetClick` _asrange_def false)
  (`BlackboardComponent.SetValueAsBool` (`AIBlueprintHelperLibrary.GetBlackboard` (`self.GetController`)) (`self.RoundStarted`) true))

(event `self.ReceiveTick`
  (params (DeltaSeconds :type "Float (single-precision)"))
  (bind _range (`self.Range`))
  (if (`/Game/Blueprints/ActorComponents/Clickable.WasClicked` (`self.ShowRange`))
    (bind _asrange_def (cast `/Game/Blueprints/Tower/Range/RangeDef` (`ChildActorComponent.ChildActor` _range)))
    (if (`SceneComponent.bVisible` _range)
      (`SceneComponent.SetVisibility` _range false false)
      (`/Game/Blueprints/Tower/Range/RangeDef.SetClick` _asrange_def false)
      (`self.UpdateTarget`)
      (else
        (`SceneComponent.SetVisibility` _range true false)
        (`/Game/Blueprints/Tower/Range/RangeDef.SetClick` _asrange_def true)))))

(fn `UserConstructionScript`)