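; MoneyTower is a tower that generates gold for the player at a regular interval while a round is running.
; Tick accumulates delta time whenever RoundIsGoing is true and compares it to TimeBetween.
; When the interval is reached, it casts player pawn 0 to CharCont, calls AddGold with GoldToAdd and resets the timer.
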(event `self.ReceiveTick`
  (params (DeltaSeconds :type "Float (single-precision)"))
  (if (`self.RoundIsGoing`)
    (bind _output_get (set `self.CurrentTime` (+ DeltaSeconds (`self.CurrentTime`))))
    (if (>= _output_get (`self.TimeBetween`))
      (bind _aschar_cont (cast `/Game/Blueprints/CharacterController/CharCont` (`GameplayStatics.GetPlayerPawn` 0)))
      (`/Game/Blueprints/CharacterController/CharCont.AddGold` _aschar_cont (`self.GoldToAdd`))
      (set `self.CurrentTime` 0.0))))

(fn `UserConstructionScript`)