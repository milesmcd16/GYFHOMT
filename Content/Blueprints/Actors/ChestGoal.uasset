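; ChestGoal is a treasure chest actor that enemies try to reach, costing the player when they do.
; On BeginPlay it writes its Box location to the Blackboard's Goal key and caches the player's CharCont pawn.
; When an EnemyABSTRACT overlaps the Box, it decrements Treasure, updates the Money text, destroys the enemy and reduces player Health.
; The construction script sets the starting Treasure and its displayed text.
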(event `self.ReceiveBeginPlay`
  (`BlackboardComponent.SetValueAsVector` (`self.Blackboard`) (`self.Goal`) (`SceneComponent.K2_GetComponentLocation` (`self.Box`)))
  (bind _aschar_cont (cast `/Game/Blueprints/CharacterController/CharCont` (`GameplayStatics.GetPlayerPawn` 0)))
  (set `self.PlayerRef` _aschar_cont))

(event `self.Box.OnComponentBeginOverlap`
  (params (OverlappedComponent :type "PrimitiveComponent Object Reference") (OtherActor :type "Actor Object Reference") (OtherComp :type "PrimitiveComponent Object Reference") (OtherBodyIndex :type Integer) (bFromSweep :type Boolean) (SweepResult :type "HitResult Structure (by ref)"))
  (bind _playerref (`self.PlayerRef`))
  (bind _asenemy_abstract (cast `/Game/Blueprints/Enemies/Actors/EnemyABSTRACT` OtherActor))
  (bind _output_get (set `self.Treasure` (- (`self.Treasure`) 1.0)))
  (`TextRenderComponent.K2_SetText` (`self.Money`) (`KismetTextLibrary.Conv_DoubleToText` _output_get "HalfToEven"))
  ;[1 1 1] when the chest is touched by an enemy, destroy enemy actor and subtract from player health
  (`self.K2_DestroyActor` _asenemy_abstract)
  (set `/Game/Blueprints/CharacterController/CharCont.Health` (- (`/Game/Blueprints/CharacterController/CharCont.Health` _playerref) 10.0) _playerref))

(fn `UserConstructionScript`
  (bind _output_get (set `self.Treasure` 50.0))
  (`TextRenderComponent.K2_SetText` (`self.Money`) (`KismetTextLibrary.Conv_DoubleToText` _output_get "HalfToEven")))