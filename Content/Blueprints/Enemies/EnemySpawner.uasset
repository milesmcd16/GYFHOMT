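; Enemy spawner actor that spawns AI squads around itself and tracks the spawned enemies.
; BeginPlay writes the mesh's location to the blackboard's Home key and builds a squad of one enemy type.
; SpawnEnemy spawns a chosen squad with a shared behavior tree at random X offsets, storing each enemy.
; Tick removes invalid entries and opens the "Test" level whenever it finds one, without checking whether the array is empty.
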(event `self.ReceiveTick`
  (params (DeltaSeconds :type "Float (single-precision)"))
  (bind _arrayofenemies (`self.ArrayOfEnemies`))
  (for _array_element _arrayofenemies
    (if (not (`KismetSystemLibrary.IsValid` _array_element))
      (`KismetArrayLibrary.Array_RemoveItem` _arrayofenemies _array_element)
      (`GameplayStatics.OpenLevel` "Test"))))

(event `self.ReceiveBeginPlay`
  (bind _mainbb (`self.MainBB`))
  (bind _home (`self.Home`))
  (`BlackboardComponent.SetValueAsVector` _mainbb _home (`SceneComponent.K2_GetComponentLocation` (`self.StaticMesh`)))
  (`KismetSystemLibrary.PrintString` (`KismetStringLibrary.Conv_VectorToString` (`BlackboardComponent.GetValueAsVector` _mainbb _home)))
  (`KismetArrayLibrary.Array_Add` (`self.Squads`) (make `/Game/Blueprints/Enemies/Squads/Squad` (`|MakeArray` "/Game/Blueprints/Enemies/Actors/Enemy1.Enemy1_C" "/Game/Blueprints/Enemies/Actors/Enemy1.Enemy1_C" "/Game/Blueprints/Enemies/Actors/Enemy1.Enemy1_C" "/Game/Blueprints/Enemies/Actors/Enemy1.Enemy1_C" "/Game/Blueprints/Enemies/Actors/Enemy1.Enemy1_C" "/Game/Blueprints/Enemies/Actors/Enemy1.Enemy1_C" "/Game/Blueprints/Enemies/Actors/Enemy1.Enemy1_C" :!type "/Game/Blueprints/Enemies/Actors/EnemyABSTRACT Class Reference"))))

(event `SpawnEnemy`
  (params (ToSpawn :type Integer))
  (for _array_element (`.EnemyList_3_9301CD2443C088E7D63738955207594B` (break `/Game/Blueprints/Enemies/Squads/Squad` (`|GetArrayItem` (`self.Squads`) ToSpawn)))
    (bind _returnvalue (`AIBlueprintHelperLibrary.SpawnAIFromClass` _array_element "/Game/Blueprints/Enemies/AI/EnemyBT1.EnemyBT1" (`KismetMathLibrary.MakeVector` (+ (`KismetMathLibrary.Conv_IntToDouble` (`KismetMathLibrary.RandomIntegerInRange` -150 150)) (.x (.location (`self.GetTransform`)))) (.y (.location (`self.GetTransform`))) (.z (.location (`self.GetTransform`)))) (.rotation (`self.GetTransform`)) false null))
    (bind _asenemy_abstract (cast `/Game/Blueprints/Enemies/Actors/EnemyABSTRACT` _returnvalue))
    (`KismetArrayLibrary.Array_Add` (`self.ArrayOfEnemies`) _asenemy_abstract)))

(fn `ArrayIsEmpty`
  (returns (isEmpty :type Boolean))
  (return (== (`KismetArrayLibrary.Array_Length` (`self.ArrayOfEnemies`)) 0)))

(fn `RemoveActor`)

(fn `UserConstructionScript`)