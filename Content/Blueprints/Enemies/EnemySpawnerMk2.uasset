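; Enemy spawner, driven through its controller's Blackboard, that sets up squad-based enemy waves per round.
; BeginPlay fills Squads with preset mixes of Enemy1 and Enemy2 and zeroes the NumberOfSquads and MaxSquadNumber keys.
; The enemiestospawnya event scales NumberOfSquads with the Round number and sets a fixed MaxSquadNumber.
; The graph contains no spawn logic itself, only the squad data and Blackboard writes.
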(event `enemiestospawnya`
  (params (`round#` :type Integer))
  (bind _returnvalue (`AIBlueprintHelperLibrary.GetBlackboard` (`self.GetController`)))
  (`BlackboardComponent.SetValueAsInt` _returnvalue (`self.NumberOfSquads`) (* `round#` 4))
  (`BlackboardComponent.SetValueAsInt` _returnvalue (`self.MaxSquadNumber`) 3))

(event `self.ReceiveBeginPlay`
  (bind _returnvalue (`AIBlueprintHelperLibrary.GetBlackboard` (`self.GetController`)))
  (`KismetArrayLibrary.Array_Add` (`self.Squads`) (make `/Game/Blueprints/Enemies/Squads/Squad` (`|MakeArray` "/Game/Blueprints/Enemies/Actors/Enemy1.Enemy1_C" "/Game/Blueprints/Enemies/Actors/Enemy1.Enemy1_C" "/Game/Blueprints/Enemies/Actors/Enemy1.Enemy1_C" "/Game/Blueprints/Enemies/Actors/Enemy1.Enemy1_C" :!type "/Game/Blueprints/Enemies/Actors/EnemyABSTRACT Class Reference")))
  (`KismetArrayLibrary.Array_Add` (`self.Squads`) (make `/Game/Blueprints/Enemies/Squads/Squad` (`|MakeArray` "/Game/Blueprints/Enemies/Actors/Enemy1.Enemy1_C" "/Game/Blueprints/Enemies/Actors/Enemy2.Enemy2_C" "/Game/Blueprints/Enemies/Actors/Enemy1.Enemy1_C" "/Game/Blueprints/Enemies/Actors/Enemy2.Enemy2_C" "/Game/Blueprints/Enemies/Actors/Enemy1.Enemy1_C" :!type "/Game/Blueprints/Enemies/Actors/EnemyABSTRACT Class Reference")))
  (`KismetArrayLibrary.Array_Add` (`self.Squads`) (make `/Game/Blueprints/Enemies/Squads/Squad` (`|MakeArray` "/Game/Blueprints/Enemies/Actors/Enemy1.Enemy1_C" "/Game/Blueprints/Enemies/Actors/Enemy1.Enemy1_C" "/Game/Blueprints/Enemies/Actors/Enemy1.Enemy1_C" :!type "/Game/Blueprints/Enemies/Actors/EnemyABSTRACT Class Reference")))
  (`KismetArrayLibrary.Array_Add` (`self.Squads`) (make `/Game/Blueprints/Enemies/Squads/Squad` (`|MakeArray` "/Game/Blueprints/Enemies/Actors/Enemy1.Enemy1_C" "/Game/Blueprints/Enemies/Actors/Enemy2.Enemy2_C" "/Game/Blueprints/Enemies/Actors/Enemy1.Enemy1_C" "/Game/Blueprints/Enemies/Actors/Enemy1.Enemy1_C" "/Game/Blueprints/Enemies/Actors/Enemy2.Enemy2_C" "/Game/Blueprints/Enemies/Actors/Enemy1.Enemy1_C" :!type "/Game/Blueprints/Enemies/Actors/EnemyABSTRACT Class Reference")))
  (`BlackboardComponent.SetValueAsInt` _returnvalue (`self.NumberOfSquads`) 0)
  (`BlackboardComponent.SetValueAsInt` _returnvalue (`self.MaxSquadNumber`) 0))

(fn `UserConstructionScript`)